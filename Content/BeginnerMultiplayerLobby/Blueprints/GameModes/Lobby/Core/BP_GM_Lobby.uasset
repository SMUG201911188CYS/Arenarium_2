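; Lobby game mode that moves all players from the lobby into the gameplay map.
; TravelTo_Gameplay_Level first calls ServerTravel on every stored player controller to put up loading screens.
; It then reads MAPNAME from the session's extra settings and, after a short delay, runs a ServerTravel console command for that map.
; If the setting is missing, it travels immediately to Gameplay_Level.
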(event Custom|TravelTo_Gameplay_Level
  ;[0.05098 0.05098 0.05098] Create a loading Screen on all players, then server travel to the Gameplay_Level
  (for _array_element (Variables|Default|GetAll_PlayerControllers)
    (Default|ServerTravel _array_element))
  (bind _extrasettings (Class|AdvancedSessionsLibrary|GetExtraSettings (Variables|Default|GetSession)))
  (bind _settingvalue (Class|AdvancedSessionsLibrary|GetSessionPropertyString _extrasettings "MAPNAME")
    (:Found
      (Utilities|FlowControl|Delay 2.0) ; Loading screen vis time
      (Development|ExecuteConsoleCommand (Utilities|String|Append "ServerTravel" " " _settingvalue) 0))
    (:NotFound
      (Development|ExecuteConsoleCommand "ServerTravel Gameplay_Level" 0))))

(fn ConstructionScript
  (|CallParentFunction))