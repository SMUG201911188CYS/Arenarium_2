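; Lobby HUD for a multiplayer game that creates and manages the lobby's on-screen widgets.
; On BeginPlay it creates the lobby HUD, player list and character select widgets for the owning player controller, adds them to the viewport and stores references.
; The player list and character select also join GameMenuWidgetList, and two events show or hide them through ToggleWidget.
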(event Custom|Toggle_PlayerList
  ;[0.05098 0.05098 0.05098] Toggle Widgets
  (CallFunction|ToggleWidget (Variables|References|GetWB_PlayerList)))

(event Custom|Toggle_CharacterSelect
  ;[0.05098 0.05098 0.05098] Toggle Widgets
  (CallFunction|ToggleWidget (Variables|References|GetWB_CharacterSelect)))

(event EventBeginPlay
  (|CallParentFunction)
  ;[0.05448 0.05448 0.05448] Create and add this Widget to the Viewport (Also store a reference to it)
  (bind _returnvalue (UserInterface|CreateWidget "/Game/BeginnerMultiplayerLobby/Widgets/Gameplay/Lobby/WB_HUD_Lobby.WB_HUD_Lobby_C" (Game|Player|GetOwningPlayerController)))
  (bind _output_get (Variables|References|SetWB_HUD_Lobby _returnvalue))
  (UserInterface|Viewport|AddtoViewport _output_get 0)
  ;[0.05448 0.05448 0.05448] Create and add this Widget to the Viewport and GameMenu_WidgetList (Also store a reference to it)
  (bind _returnvalue_2 (UserInterface|CreateWidget "/Game/BeginnerMultiplayerLobby/Widgets/Gameplay/PlayerList/WB_PlayerList.WB_PlayerList_C" (Game|Player|GetOwningPlayerController)))
  (bind _output_get_2 (Variables|References|SetWB_PlayerList _returnvalue_2))
  (UserInterface|Viewport|AddtoViewport _output_get_2 0)
  (Utilities|Array|Add (Variables|Default|GetGameMenu_WidgetList) (Variables|References|GetWB_PlayerList))
  ;[0.05448 0.05448 0.05448] Create and add this Widget to the Viewport and GameMenu_WidgetList (Also store a reference to it)
  (bind _returnvalue_3 (UserInterface|CreateWidget "/Game/BeginnerMultiplayerLobby/Widgets/Gameplay/Lobby/CharacterSelect/WB_CharacterSelect.WB_CharacterSelect_C" (Game|Player|GetOwningPlayerController)))
  (bind _output_get_3 (Variables|References|SetWB_CharacterSelect _returnvalue_3))
  (UserInterface|Viewport|AddtoViewport _output_get_3 0)
  (Utilities|Array|Add (Variables|Default|GetGameMenu_WidgetList) (Variables|References|GetWB_CharacterSelect)))

(fn ConstructionScript
  (|CallParentFunction))